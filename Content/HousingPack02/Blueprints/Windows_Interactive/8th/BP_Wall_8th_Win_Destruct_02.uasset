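; Interactive wall window from a housing pack whose glass pane slides open and closed when the player presses E.
; Overlapping the trigger enables input for player controller 0 and leaving disables it, with no check on the overlapping actor.
; The OpenClose timeline lerps the pane's relative location between Close and Open, playing or reversing based on IsClosed.
; Tick recomputes IsClosed from the timeline value, treating anything short of fully open as closed.
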(event OnComponentBeginOverlap(Trigger)
  (params (OverlappedComponent :type Primitive%20Component%20Object%20Reference) (OtherActor :type Actor%20Object%20Reference) (OtherComp :type Primitive%20Component%20Object%20Reference) (OtherBodyIndex :type Integer) (bFromSweep :type Boolean) (SweepResult :type Hit%20Result%20Structure%20%28by%20ref%29))
  (Input|EnableInput (Game|GetPlayerController 0)))

(event OnComponentEndOverlap(Trigger)
  (params (OverlappedComponent :type Primitive%20Component%20Object%20Reference) (OtherActor :type Actor%20Object%20Reference) (OtherComp :type Primitive%20Component%20Object%20Reference) (OtherBodyIndex :type Integer))
  (Input|DisableInput (Game|GetPlayerController 0)))

(event EventTick
  (params (DeltaSeconds :type Float%20%28single-precision%29))
  (Variables|Default|SetIs%20Closed (< (stale Input|KeyboardEvents|E _windowoperation) 1.0)))

(event Input|KeyboardEvents|E
  (params (Key :type Key%20Structure))
  (:Pressed
    (if (Variables|Default|GetIs%20Closed)
      (bind _windowoperation (Timeline|OpenClose Play)
        (:Update
          (Transformation|SetRelativeLocation (Variables|Default|GetSM_Glass_Pane_02_DM1) (Math|Vector|Lerp(Vector) (Variables|WindowSetup|GetClose) (Variables|WindowSetup|GetOpen) _windowoperation) false false)))
      (else
        (Timeline|OpenClose Reverse)))))

(fn ConstructionScript)