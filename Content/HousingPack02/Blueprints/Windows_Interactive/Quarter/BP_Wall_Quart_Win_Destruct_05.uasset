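; Housing-pack quarter wall with three interactive windows, whose glass panes the player slides open and closed with E.
; Each window's trigger enables input and sets an overlap flag, and a timeline lerps that pane's relative location between closed and open vectors.
; Tick derives closed flags from timeline values, so E reverses only a fully open pane.
; Leaving Trigger_02 clears window 3's flag instead of its own, so OverlapWin02 stays set.
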(event OnComponentBeginOverlap(Trigger_01)
  (params (OverlappedComponent :type Primitive%20Component%20Object%20Reference) (OtherActor :type Actor%20Object%20Reference) (OtherComp :type Primitive%20Component%20Object%20Reference) (OtherBodyIndex :type Integer) (bFromSweep :type Boolean) (SweepResult :type Hit%20Result%20Structure%20%28by%20ref%29))
  (Input|EnableInput (Game|GetPlayerController 0))
  (Variables|Default|SetOverlap_Win_01 true))

(event OnComponentEndOverlap(Trigger_01)
  (params (OverlappedComponent :type Primitive%20Component%20Object%20Reference) (OtherActor :type Actor%20Object%20Reference) (OtherComp :type Primitive%20Component%20Object%20Reference) (OtherBodyIndex :type Integer))
  (Input|DisableInput (Game|GetPlayerController 0))
  (Variables|Default|SetOverlap_Win_01 false))

(event OnComponentBeginOverlap(Trigger_02)
  (params (OverlappedComponent :type Primitive%20Component%20Object%20Reference) (OtherActor :type Actor%20Object%20Reference) (OtherComp :type Primitive%20Component%20Object%20Reference) (OtherBodyIndex :type Integer) (bFromSweep :type Boolean) (SweepResult :type Hit%20Result%20Structure%20%28by%20ref%29))
  (Input|EnableInput (Game|GetPlayerController 0))
  (Variables|Default|SetOverlap_Win_02 true))

(event OnComponentEndOverlap(Trigger_02)
  (params (OverlappedComponent :type Primitive%20Component%20Object%20Reference) (OtherActor :type Actor%20Object%20Reference) (OtherComp :type Primitive%20Component%20Object%20Reference) (OtherBodyIndex :type Integer))
  (Input|DisableInput (Game|GetPlayerController 0))
  (Variables|Default|SetOverlap_Win_03 false))

(event OnComponentBeginOverlap(Trigger_03)
  (params (OverlappedComponent :type Primitive%20Component%20Object%20Reference) (OtherActor :type Actor%20Object%20Reference) (OtherComp :type Primitive%20Component%20Object%20Reference) (OtherBodyIndex :type Integer) (bFromSweep :type Boolean) (SweepResult :type Hit%20Result%20Structure%20%28by%20ref%29))
  (Input|EnableInput (Game|GetPlayerController 0))
  (Variables|Default|SetOverlap_Win_03 true))

(event OnComponentEndOverlap(Trigger_03)
  (params (OverlappedComponent :type Primitive%20Component%20Object%20Reference) (OtherActor :type Actor%20Object%20Reference) (OtherComp :type Primitive%20Component%20Object%20Reference) (OtherBodyIndex :type Integer))
  (Input|DisableInput (Game|GetPlayerController 0))
  (Variables|Default|SetOverlap_Win_03 false))

(event EventTick
  (params (DeltaSeconds :type Float%20%28single-precision%29))
  (Variables|Default|SetIs%20Closed (< (stale Input|KeyboardEvents|E _windowoperation) 1.0))
  (Variables|Default|SetIs%20Closed_1 (< (stale Input|KeyboardEvents|E _newtrack_1) 1.0))
  (Variables|Default|SetIs%20Closed_2 (< (stale Input|KeyboardEvents|E _newtrack_1) 1.0)))

(event Input|KeyboardEvents|E
  (params (Key :type Key%20Structure))
  (:Pressed
    (if (Variables|Default|GetOverlap_Win_01)
      (if (Variables|Default|GetIs%20Closed)
        (bind _windowoperation (Timeline|OpenClose Play)
          (:Update
            (Transformation|SetRelativeLocation (Variables|Default|GetSM_Glass_Pane_02_DM1) (Math|Vector|Lerp(Vector) (Variables|WindowSetup|GetClose) (Variables|WindowSetup|GetOpen) _windowoperation) false false)
            (if (< _windowoperation 1.0)
              _)))
        (else
          (Timeline|OpenClose Reverse))))))

(event Input|KeyboardEvents|E
  (params (Key :type Key%20Structure))
  (:Pressed
    (if (Variables|Default|GetOverlap_Win_02)
      (if (Variables|Default|GetIs%20Closed_1)
        (bind _newtrack_1 (Timeline|Timeline_0 Play)
          (:Update
            (Transformation|SetRelativeLocation (Variables|Default|GetSM_Glass_Pane_02_DM2) (Math|Vector|Lerp(Vector) (Variables|WindowSetup|GetClose_1) (Variables|WindowSetup|GetOpen_1) _newtrack_1) false false)))
        (else
          (Timeline|Timeline_0 Reverse))))))

(event Input|KeyboardEvents|E
  (params (Key :type Key%20Structure))
  (:Pressed
    (if (Variables|Default|GetOverlap_Win_03)
      (if (Variables|Default|GetIs%20Closed_2)
        (bind _newtrack_1 (Timeline|Timeline_1 Play)
          (:Update
            (Transformation|SetRelativeLocation (Variables|Default|GetSM_Glass_Pane_02_DM3) (Math|Vector|Lerp(Vector) (Variables|WindowSetup|GetClose_2) (Variables|WindowSetup|GetOpen_2) _newtrack_1) false false)))
        (else
          (Timeline|Timeline_1 Reverse))))))

(fn ConstructionScript)