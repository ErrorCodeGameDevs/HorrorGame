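; Double garage door Blueprint that opens when something enters its trigger box and closes when it leaves.
; Box overlap events play separate open and close animations on the skeletal mesh, tracking state with PlayerIsInBox and DoorIsOpening.
; If an overlap changes mid-animation, the play rate flips to reverse or resume the current animation instead of restarting it.
; Overlaps are not filtered by actor type, despite the player-named flag.
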(event OnComponentBeginOverlap(Box)
  (params (OverlappedComponent :type Primitive%20Component%20Object%20Reference) (OtherActor :type Actor%20Object%20Reference) (OtherComp :type Primitive%20Component%20Object%20Reference) (OtherBodyIndex :type Integer) (bFromSweep :type Boolean) (SweepResult :type Hit%20Result%20Structure%20%28by%20ref%29))
  (Variables|Default|SetPlayerIsInBox true)
  (if (Audio|Components|Audio|IsPlaying (Variables|Default|GetSkeletalMeshComponent0))
    (if (Variables|Default|GetDoorIsOpening)
      (Components|Timeline|SetPlayRate (Variables|Default|GetSkeletalMeshComponent0) 1.0)
      (else
        (Components|Timeline|SetPlayRate (Variables|Default|GetSkeletalMeshComponent0) -1.0)))
    (else
      (Components|Timeline|SetPlayRate (Variables|Default|GetSkeletalMeshComponent0) 1.0)
      (Components|Animation|PlayAnimation (Variables|Default|GetSkeletalMeshComponent0) "/Game/HousingPack02/Animations/SK_Garage_Double_01_Open_Anim.SK_Garage_Double_01_Open_Anim" false)
      (Variables|Default|SetDoorIsOpening true))))

(event OnComponentEndOverlap(Box)
  (params (OverlappedComponent :type Primitive%20Component%20Object%20Reference) (OtherActor :type Actor%20Object%20Reference) (OtherComp :type Primitive%20Component%20Object%20Reference) (OtherBodyIndex :type Integer))
  (if (Audio|Components|Audio|IsPlaying (Variables|Default|GetSkeletalMeshComponent0))
    (if (Variables|Default|GetDoorIsOpening)
      (Components|Timeline|SetPlayRate (Variables|Default|GetSkeletalMeshComponent0) -1.0)
      (Variables|Default|SetPlayerIsInBox false)
      (else
        (Components|Timeline|SetPlayRate (Variables|Default|GetSkeletalMeshComponent0) 1.0)
        (Variables|Default|SetPlayerIsInBox false)))
    (elif (Variables|Default|GetPlayerIsInBox)
      (Components|Timeline|SetPlayRate (Variables|Default|GetSkeletalMeshComponent0) 1.0)
      (Components|Animation|PlayAnimation (Variables|Default|GetSkeletalMeshComponent0) "/Game/HousingPack02/Animations/SK_Garage_Double_01_Close_Anim.SK_Garage_Double_01_Close_Anim" false)
      (Variables|Default|SetPlayerIsInBox false)
      (Variables|Default|SetDoorIsOpening false))))

(fn ConstructionScript)