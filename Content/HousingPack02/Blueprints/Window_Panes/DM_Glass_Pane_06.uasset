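; Destructible glass window pane from a housing pack that reacts to hits from first-person projectiles.
; On a projectile hit, it checks the IsStacked5 counter and increments it while it is negative.
; Once the counter is zero or higher, it turns off physics simulation on the Destructible component and applies small radial damage at the impact point, with the projectile as damage causer.
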(event OnComponentHit(Destructible)
  (params (HitComponent :type Primitive%20Component%20Object%20Reference) (OtherActor :type Actor%20Object%20Reference) (OtherComp :type Primitive%20Component%20Object%20Reference) (NormalImpulse :type Vector :default "0, 0, 0") (Hit :type Hit%20Result%20Structure%20%28by%20ref%29))
  (bind _asbp_first_person_projectile (Utilities|Casting|CastToBP_FirstPersonProjectile OtherActor))
  (if (>= (Variables|Default|GetisStacked5?) 0.0)
    (Physics|SetSimulatePhysics (Variables|Default|GetDestructible) false)
    (Game|Damage|ApplyRadialDamage 1.0 (.ImpactPoint (Collision|BreakHitResult Hit)) 1.0 "/Script/Engine.DamageType" 0 _asbp_first_person_projectile 0 true "ECC_Visibility")
    (else
      (Variables|Default|SetisStacked5? (+ (Variables|Default|GetisStacked5?) 1.0)))))

(fn ConstructionScript)